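; BP_Enemy is an enemy Blueprint whose only active event logic prints incoming damage amounts to the screen.
; Code that would link its HealthBarWidget's WBP_HealthBar to the enemy is present but disconnected, and BeginPlay is empty.
; IsWeaponEquipped resolves the active hotbar slot through Inventory to a DT_Items row and tests whether its item type is the first enumerator.
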(event Game|Damage|EventAnyDamage
  (params (Damage :type Float%20%28single-precision%29) (DamageType :type Damage%20Type%20Object%20Reference) (InstigatedBy :type Controller%20Object%20Reference) (DamageCauser :type Actor%20Object%20Reference))
  (Development|PrintString (Utilities|String|ToString(Float) Damage)))

(event EventBeginPlay)

(fn ConstructionScript)

(fn IsWeaponEquipped
  (bind _activehotbarindex (Variables|Default|GetActiveHotbarIndex))
  (bind _hotbaritems (Variables|Default|GetHotbarItems))
  (bind _output (Utilities|Array|Get(acopy) _hotbaritems _activehotbarindex))
  (if (> _output -1)
    (bind _returnvalue (Utilities|GetDataTableRow "/Game/Items/DT_Items.DT_Items" (.rowname (.Item (Utilities|Struct|BreakST_InventorySlot (Utilities|Array|Get(acopy) (Variables|Default|GetInventory) _output)))))
      (:then
        (return (Utilities|Enum|Equal(Enum) (.ItemType (Utilities|Struct|BreakST_ItemStats _returnvalue)) "NewEnumerator0"))))))